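; Game mode for the day phase, which runs a timed day and then loads the kitchen level for night.
; BeginPlay creates the HUD and adds dash, attack and buff components to the BP_BakerDay player pawn at runtime, keeping references to each.
; Tick accumulates elapsed time, prints it on screen, and calls EndOfDay to open LVL_Kitchen once DayDuration is reached.
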(event `self.ReceiveBeginPlay`
  (bind _returnvalue (`|GenericCreateObject` "/Game/05_BP/06_UI/WBP_Hud.WBP_Hud_C"))
  (bind _output_get (set `self.HudWidget` _returnvalue))
  (set `Widget.RenderOpacity` 1.0 _output_get)
  (`UserWidget.AddToViewport` _output_get 0)
  (bind _asbp_baker_day (cast `/Game/05_BP/01_Player/BP_BakerDay` (`GameplayStatics.GetPlayerPawn` 0))
    (:`then`
      (bind _output_get_2 (set `self.Character` _asbp_baker_day))
      (bind _returnvalue_2 (`|AddComponentByClass` _output_get_2 "/Game/05_BP/01_Player/ActorComponent/AC_BP_Dash.AC_BP_Dash_C"))
      (set `self.DashComponent` _returnvalue_2)
      (bind _returnvalue_3 (`|AddComponentByClass` (`self.Character`) "/Game/05_BP/01_Player/ActorComponent/AC_BP_Attack.AC_BP_Attack_C"))
      (set `self.AttackComponent` _returnvalue_3)
      (bind _returnvalue_4 (`|AddComponentByClass` (`self.Character`) "/Game/05_BP/01_Player/ActorComponent/AC_BP_Buff.AC_BP_Buff_C"))
      (set `self.BuffComponent` _returnvalue_4))
    (:`CastFailed`
      (`KismetSystemLibrary.PrintString` "Failed to Baker Day" true true (struct :`R` 1.0 :`A` 1.0) 5.0))))

(event `self.ReceiveTick`
  (params (DeltaSeconds :type "Float (single-precision)"))
  (bind _output_get (set `self.Time` (+ DeltaSeconds (`self.Time`))))
  (`KismetSystemLibrary.PrintString` (`KismetStringLibrary.TimeSecondsToString` _output_get) true false (struct :`G` 0.66 :`B` 1.0 :`A` 1.0) 0.0)
  (if (>= (`self.Time`) (`self.DayDuration`))
    (`self.EndOfDay`)))

(event `EndOfDay`
  (`KismetSystemLibrary.PrintString` "Switch to night" true true (struct :`G` 0.181056 :`B` 1.0 :`A` 1.0) 5.0)
  (`GameplayStatics.OpenLevelBySoftObjectPtr` "/Game/07_Levels/LevelKitchen/LVL_Kitchen.LVL_Kitchen"))

(fn `UserConstructionScript`)