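; BP_Enemy_Melee is a sword-wielding enemy that overrides attack, equip and unequip events from its parent.
; Attack plays a slash montage whose notify runs a short forward sphere trace to damage a pawn, then signals attack end on completion or interruption.
; Equip only sets the wielding flag and fires its callback, as the sword spawn-and-attach code is disconnected.
; Unequip plays a sheath montage that destroys the weapon on notify.
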(event `self.ReceiveBeginPlay`
  (`parent.ReceiveBeginPlay`))

(event `/Game/05_BP/04_Enemies/AI/BPI_EnemyAI.Attack`
  (bind _returnvalue (`self.K2_GetActorLocation`))
  (bind _notifyname (`|PlayMontage` (`self.Mesh`) "/Game/leBaguette/Paul/AnimManny/Montage_Sword_Slash.Montage_Sword_Slash")
    (:`OnCompleted`
      (`self.OnAttackEnd` :!label _label))
    (:`OnInterrupted`
      (goto _label))
    (:`OnNotifyBegin`
      (switch `name` _notifyname
        (:`Slash`
          (bind (_outhit _returnvalue_2) (`KismetSystemLibrary.SphereTraceSingleForObjects` :`Start` _returnvalue :`End` (+ _returnvalue (* (`self.GetActorForwardVector`) 200.0)) :`Radius` 20.0 :`ObjectTypes` (`|MakeArray` "ObjectTypeQuery3" :!type "EObjectTypeQuery Enum") :`DrawDebugType` "ForDuration"))
          (if _returnvalue_2
            (`GameplayStatics.ApplyDamage` (`.HitActor` (`GameplayStatics.BreakHitResult` _outhit)) 25.0 null self)))))))

(event `/Game/05_BP/04_Enemies/AI/BPI_EnemyAI.EquipWeapon`
  (set `self.isWieldingWeapon` true)
  (`self.OnWeaponEquiped`))

(event `/Game/05_BP/04_Enemies/AI/BPI_EnemyAI.UnequipWeapon`
  (bind _notifyname (`|PlayMontage` (`self.Mesh`) "/Game/05_BP/04_Enemies/Anim/Montage_Sheath_Sword.Montage_Sheath_Sword")
    (:`OnCompleted`
      (`self.OnWeaponUnequipped`))
    (:`OnNotifyBegin`
      (switch `name` _notifyname
        (:`DropSword`
          (`self.K2_DestroyActor` (`self.WeaponActor`))
          (set `self.isWieldingWeapon` false))))))

(fn `UserConstructionScript`
  (`parent.UserConstructionScript`))