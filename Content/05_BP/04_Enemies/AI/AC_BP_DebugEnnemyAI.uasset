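; Debug component for enemy AI that toggles an enemy between attacking and passive states with the T key.
; On each press it finds a single BP_Enemy_Base in the world and casts its controller to AIC_Ennemy_Base.
; A FlipFlop alternates between setting the attacking state, passing the component's owner, and the passive state.
; BeginPlay caches the BP_BakerDay player character, though the toggle does not use it.
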(event `self.ReceiveBeginPlay`
  (bind _asbp_baker_day (cast `/Game/05_BP/01_Player/BP_BakerDay` (`GameplayStatics.GetPlayerCharacter` 0)))
  (set `self.As BP Baker Day` _asbp_baker_day))

(event `Key|T`
  (params (Key :type "Key Structure"))
  (:`Pressed`
    (bind _returnvalue (`GameplayStatics.GetActorOfClass` "/Game/05_BP/04_Enemies/BP_Enemy_Base.BP_Enemy_Base_C"))
    (bind _asaic_ennemy_base (cast `/Game/05_BP/04_Enemies/AI/AIC_Ennemy_Base` (`AIBlueprintHelperLibrary.GetAIController` _returnvalue)))
    (`/Engine/EditorBlueprintResources/StandardMacros.FlipFlop`
      (:`A`
        (`/Game/05_BP/04_Enemies/AI/AIC_Ennemy_Base.SetStateHasAttacking` _asaic_ennemy_base (`self.GetOwner`)))
      (:`B`
        (`/Game/05_BP/04_Enemies/AI/AIC_Ennemy_Base.SetStateHasPassive` _asaic_ennemy_base)))))