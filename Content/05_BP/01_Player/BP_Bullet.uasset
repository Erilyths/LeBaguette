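; BP_Bullet is a player projectile that damages what its collider overlaps.
; Init stores the damage and initial direction, though these graphs never read the direction.
; On overlap, any actor other than the player character that implements BPI_Attack receives ApplyDamage, and the bullet destroys itself.
; The SetLifeSpan call is disconnected, so the Lifetime value is never applied here.
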(event `self.ReceiveBeginPlay`)

(event `self.Collider.OnComponentBeginOverlap`
  (params (OverlappedComponent :type "PrimitiveComponent Object Reference") (OtherActor :type "Actor Object Reference") (OtherComp :type "PrimitiveComponent Object Reference") (OtherBodyIndex :type Integer) (bFromSweep :type Boolean) (SweepResult :type "HitResult Structure (by ref)"))
  (if (and (!= OtherActor (`GameplayStatics.GetPlayerCharacter` 0)) (`KismetSystemLibrary.DoesImplementInterface` OtherActor "/Game/05_BP/01_Player/Interface/BPI_Attack.BPI_Attack_C"))
    (`self.Attack` OtherActor)
    (`self.K2_DestroyActor`)))

(fn `Attack`
  (params (ActorToAttack :type "Actor Object Reference"))
  (`GameplayStatics.ApplyDamage` ActorToAttack (`self.Damage`)))

(fn `Init`
  (params (Damage :type "Float (double-precision)") (InitialDir :type "Vector Structure"))
  (set `self.Damage` Damage)
  (set `self.Initial Dir` InitialDir))

(fn `UserConstructionScript`)