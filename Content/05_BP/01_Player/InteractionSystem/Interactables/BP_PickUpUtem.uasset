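; Interactable pickup actor that plays a tone at its location and destroys itself when an interactor uses it.
; Interact only prints an "added to inventory" message naming the item and interactor; no inventory data is changed.
; Interaction getters expose type and hold duration from variables, while tap count is hardcoded and prompt and location return empty or zero values.
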(event `/Game/05_BP/01_Player/InteractionSystem/BPI_Interactable.Interact`
  (params (Interactor :type "Actor Object Reference"))
  (`KismetSystemLibrary.PrintString` (`KismetTextLibrary.Conv_TextToString` (`|FormatText` "Added {itemName} to the inventory of {ActorName}" (`KismetSystemLibrary.GetDisplayName` self) (`KismetSystemLibrary.GetDisplayName` Interactor))))
  (`GameplayStatics.PlaySoundAtLocation` "/Engine/EngineSounds/1kSineTonePing.1kSineTonePing" (`self.K2_GetActorLocation`) (struct) 1.0 1.0 0.0 null null null null)
  (`self.K2_DestroyActor`))

(fn `GetHoldDuration`
  (returns (Duration :type "Float (double-precision)"))
  (return (`self.HoldDuration`)))

(fn `GetInteractionLocation`
  (returns (`Location ` :type "Vector Structure"))
  (return (0.0 0.0 0.0)))

(fn `GetInteractionPrompt`
  (returns (Value :type Text))
  (return ""))

(fn `GetInteractionType`
  (returns (Type :type "/Game/05_BP/01_Player/InteractionSystem/E_InteractionTypes Enum"))
  (return (`self.InteractionType`)))

(fn `GetTapCount`
  (returns (Value :type Integer))
  (return 4))

(fn `UserConstructionScript`)