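; Player health actor component that tracks current HP, starting it at MaxHp on BeginPlay.
; TakeDamage scales incoming damage linearly by DefenseModifier, where values above one reduce it, then returns a death flag, damage taken and new HP.
; Heal adds HP capped at MaxHp, while damage has no lower clamp.
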(event `self.ReceiveBeginPlay`
  (set `self.CurrentHp` (`self.MaxHp`)))

(fn `Heal`
  (params (Amount :type "Float (double-precision)"))
  (returns (NewHP :type "Float (double-precision)"))
  (bind _maxhp (`self.MaxHp`))
  (bind _returnvalue (+ Amount (`self.CurrentHp`)))
  (bind _output_get (set `self.CurrentHp` (`KismetMathLibrary.SelectFloat` _returnvalue _maxhp (<= _returnvalue _maxhp))))
  (return _output_get))

(fn `TakeDamage`
  (params (Damage :type "Float (double-precision)"))
  (returns (Died :type Boolean) (DamageTook :type "Float (double-precision)") (NewHp :type "Float (double-precision)"))
  (locals (TrueDamage :type "Float (double-precision)"))
  (bind _output_get (set `local.TrueDamage` (* Damage (- 1.0 (- (* (`self.DefenseModifier`) 1.0) 1.0)))))
  (bind _output_get_2 (set `self.CurrentHp` (- (`self.CurrentHp`) _output_get)))
  (return (<= _output_get_2 0.0) (`local.TrueDamage`) _output_get_2))