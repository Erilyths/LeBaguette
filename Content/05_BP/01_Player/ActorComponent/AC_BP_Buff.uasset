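; Actor component that manages timed buffs for the day-phase baker player, affecting healing, attack speed, move speed, damage, luck and defense.
; AddBuff applies a new buff's effect and stores its timer in a map; re-adding only resets the timer.
; Tick counts timers down and reverts expired buffs.
; Modifiers stack by multiplication on the attack, health, character or game mode, and the B key grants BarleySugar.
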(event `AddBuff`
  (params (Buff :type "/Game/05_BP/01_Player/DataAssets/Inventory/Da_Buff Object Reference"))
  (bind _activebuffs (`self.ActiveBuffs`))
  (if (not (`BlueprintMapLibrary.Map_Contains` _activebuffs Buff))
    (`self.UpdateBuff` Buff "/Game/05_BP/01_Player/DataAssets/Inventory/Buffs/Buff_Default.Buff_Default"))
  (`BlueprintMapLibrary.Map_Add` _activebuffs Buff (`/Game/05_BP/01_Player/DataAssets/Inventory/Da_Buff.Time` Buff)))

(event `self.ReceiveTick`
  (params (DeltaSeconds :type "Float (single-precision)"))
  (`self.UpdateBuffTimers` DeltaSeconds))

(event `self.ReceiveBeginPlay`
  (bind _asbp_baker_day (cast `/Game/05_BP/01_Player/BP_BakerDay` (`GameplayStatics.GetPlayerPawn` 0)))
  (set `self.Character` _asbp_baker_day)
  (bind _asbp_game_mode_day (cast `/Game/05_BP/05_GameMode/BP_GameModeDay` (`GameplayStatics.GetGameMode`)))
  (set `self.GameMode` _asbp_game_mode_day)
  (set `self.AttackComponent` (`Actor.GetComponentByClass` (`self.Character`) "/Game/05_BP/01_Player/ActorComponent/AC_BP_Attack.AC_BP_Attack_C"))
  (set `self.HealthComponent` (`Actor.GetComponentByClass` (`self.Character`) "/Game/05_BP/01_Player/ActorComponent/AC_BP_Heallth.AC_BP_Heallth_C")))

(event `Key|B`
  (params (Key :type "Key Structure"))
  (:`Pressed`
    (`self.AddBuff` "/Game/05_BP/01_Player/DataAssets/Inventory/Buffs/Buff_BarleySugar.Buff_BarleySugar")))

(fn `AddBuffOnTargetFloat`
  (params (TargetFloat :type "Float (double-precision) (by ref)") (NewBuffValue :type "Float (double-precision)"))
  (if (== TargetFloat 1.0)
    (`|VariableSetRef` TargetFloat NewBuffValue)
    (else
      (`|VariableSetRef` TargetFloat (* TargetFloat NewBuffValue)))))

(fn `RemoveBuffOnTargetFloat`
  (params (TargetFloat :type "Float (double-precision) (by ref)") (OldBuffValue :type "Float (double-precision)"))
  (if (== TargetFloat OldBuffValue)
    (`|VariableSetRef` TargetFloat 1.0)
    (else
      (`|VariableSetRef` TargetFloat (/ TargetFloat OldBuffValue)))))

(fn `UpdateBuff`
  (params (NewBuffs :type "/Game/05_BP/01_Player/DataAssets/Inventory/Da_Buff Object Reference") (BuffToRemove :type "/Game/05_BP/01_Player/DataAssets/Inventory/Da_Buff Object Reference"))
  (bind _attackcomponent (`self.AttackComponent`))
  (bind _healthcomponent (`self.HealthComponent`))
  (bind _attackcomponent_2 (`self.AttackComponent`))
  (bind _value (`/Game/05_BP/01_Player/DataAssets/Inventory/Da_Buff.Value` (`local.NewBuffs`)))
  (bind _value_2 (`/Game/05_BP/01_Player/DataAssets/Inventory/Da_Buff.Value` (`local.BuffToRemove`)))
  (switch `/Game/05_BP/01_Player/Struct/Enum_BuffType` (`/Game/05_BP/01_Player/DataAssets/Inventory/Da_Buff.BuffType` (`local.NewBuffs`))
    (:`NewEnumerator7`
      _)
    (:`NewEnumerator0`
      (`/Game/05_BP/01_Player/ActorComponent/AC_BP_Heallth.Heal` _healthcomponent _value))
    (:`NewEnumerator1`
      (`self.AddBuffOnTargetFloat` (`/Game/05_BP/01_Player/ActorComponent/AC_BP_Attack.AttackRateModifier` _attackcomponent) _value))
    (:`NewEnumerator2`
      (`self.AddBuffOnTargetFloat` (`/Game/05_BP/01_Player/BP_BakerDay.SpeedModifier` (`self.Character`)) _value)
      (`/Game/05_BP/01_Player/BP_BakerDay.UpdateBuffs` (`self.Character`)))
    (:`NewEnumerator3`
      (`self.AddBuffOnTargetFloat` (`/Game/05_BP/01_Player/ActorComponent/AC_BP_Attack.DamageBonus` _attackcomponent) _value))
    (:`NewEnumerator4`
      (`self.AddBuffOnTargetFloat` (`/Game/05_BP/05_GameMode/BP_GameModeDay.Luck` (`self.GameMode`)) _value))
    (:`NewEnumerator5`
      (`self.AddBuffOnTargetFloat` (`/Game/05_BP/01_Player/ActorComponent/AC_BP_Heallth.DefenseModifier` _healthcomponent) _value)))
  (switch `/Game/05_BP/01_Player/Struct/Enum_BuffType` (`/Game/05_BP/01_Player/DataAssets/Inventory/Da_Buff.BuffType` (`local.BuffToRemove`))
    (:`NewEnumerator7`
      _)
    (:`NewEnumerator0`
      _)
    (:`NewEnumerator1`
      (`self.RemoveBuffOnTargetFloat` (`/Game/05_BP/01_Player/ActorComponent/AC_BP_Attack.AttackRateModifier` _attackcomponent_2) _value_2))
    (:`NewEnumerator2`
      (`self.RemoveBuffOnTargetFloat` (`/Game/05_BP/01_Player/BP_BakerDay.SpeedModifier` (`self.Character`)) _value_2)
      (`/Game/05_BP/01_Player/BP_BakerDay.UpdateBuffs` (`self.Character`)))
    (:`NewEnumerator3`
      (`self.RemoveBuffOnTargetFloat` (`/Game/05_BP/01_Player/ActorComponent/AC_BP_Attack.DamageBonus` _attackcomponent_2) _value_2))
    (:`NewEnumerator4`
      (`self.RemoveBuffOnTargetFloat` (`/Game/05_BP/05_GameMode/BP_GameModeDay.Luck` (`self.GameMode`)) _value_2))
    (:`NewEnumerator5`
      (`self.RemoveBuffOnTargetFloat` (`/Game/05_BP/01_Player/ActorComponent/AC_BP_Heallth.DefenseModifier` (`self.HealthComponent`)) _value_2)))
  (return))

(fn `UpdateBuffTimers`
  (params (DeltaTime :type "Float (double-precision)"))
  (bind _activebuffs (`self.ActiveBuffs`))
  (bind (_keypin _valuepin) (`|MapForEach` (`self.ActiveBuffs`))
    (:`then`
      (bind _returnvalue (- _valuepin (`local.DeltaTime`)))
      (if (<= _returnvalue 0.0)
        (`self.UpdateBuff` "/Game/05_BP/01_Player/DataAssets/Inventory/Buffs/Buff_Default.Buff_Default" _keypin)
        (`BlueprintMapLibrary.Map_Remove` _activebuffs _keypin)
        (else
          (`BlueprintMapLibrary.Map_Add` _activebuffs _keypin _returnvalue))))))