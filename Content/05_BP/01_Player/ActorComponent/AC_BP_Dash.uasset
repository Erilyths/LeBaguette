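; Actor component for the BakerDay player character that handles a charge-limited dash on the IA_Jump input.
; BeginPlay caches the baker and day game mode and loads max charges from the baker's metrics data asset.
; The input only spends a charge when dashing is allowed.
; The launch along capsule forward, state switches, cooldown recharge and HUD update are disconnected, so they never run.
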(event `self.ReceiveBeginPlay`
  (bind _asbp_baker_day (cast `/Game/05_BP/01_Player/BP_BakerDay` (`self.GetOwner`)))
  (set `self.BakerRef` _asbp_baker_day)
  (set `self.DashCount` (`/Game/05_BP/01_Player/DataAssets/DA_BakerDayMetrics.MaxDashCount` (`/Game/05_BP/01_Player/BP_BakerDay.MetricsDataAsset` (`self.BakerRef`))))
  (bind _asbp_game_mode_day (cast `/Game/05_BP/05_GameMode/BP_GameModeDay` (`GameplayStatics.GetGameMode`))
    (:`then`
      (set `self.Game Mode` _asbp_game_mode_day))
    (:`CastFailed`
      (`KismetSystemLibrary.PrintString` "Failed to Cast Game Mode Day (maybe using baker day without gamemode day)" true true (struct :`R` 1.0 :`A` 1.0) 5.0))))

(event `EnhancedInput|/Game/05_BP/03_Input/Actions/IA_Jump`
  (params (ActionValue :type Boolean) (ElapsedSeconds :type "Float (double-precision)") (TriggeredSeconds :type "Float (double-precision)") (InputAction :type "InputAction Object Reference" :default "/Game/05_BP/03_Input/Actions/IA_Jump.IA_Jump"))
  ; Dash
  (:`Triggered`
    (if (and (>= (`self.DashCount`) 1) (`/Game/05_BP/01_Player/BP_BakerDay.canDash` (`self.BakerRef`)))
      (`/Engine/EditorBlueprintResources/StandardMacros.DecrementInt` (`self.DashCount`)))))