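; Player inventory component that stores buffs, ingredients and weapons, plus three equipped buff slots.
; Buffs and ingredients are maps of counts, while weapons are a list; functions add, remove, query and equip items.
; Changes call per-category update dispatchers with the current data for listeners.
; Removal subtracts counts without clamping or deleting entries, and RemoveWeapon's inverted check only calls Remove when the weapon is absent.
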(fn `AddBuff`
  (params (Buff :type "/Game/05_BP/01_Player/DataAssets/Inventory/Da_Buff Object Reference (by ref)") (Number :type Integer :default 1))
  (bind _buffs (`self.Buffs`))
  (bind _buff (`local.Buff`))
  (bind (_value _returnvalue) (`BlueprintMapLibrary.Map_Find` (`self.Buffs`) Buff))
  (if _returnvalue
    (`BlueprintMapLibrary.Map_Add` _buffs _buff (+ _value Number))
    (else
      (`BlueprintMapLibrary.Map_Add` _buffs _buff Number)))
  (`self.OnUpdatedBuffs` (`self.Buffs`) (`self.BuffSlot1`) (`self.BuffSlot2`) (`self.BuffSlot3`)))

(fn `AddIngredient`
  (params (Ingredient :type "/Game/05_BP/01_Player/DataAssets/Inventory/DA_Item Object Reference (by ref)") (Number :type Integer :default 1))
  (bind _ingredients (`self.Ingredients`))
  (bind _ingredient (`local.Ingredient`))
  (bind (_value _returnvalue) (`BlueprintMapLibrary.Map_Find` (`self.Ingredients`) Ingredient))
  (if _returnvalue
    (`BlueprintMapLibrary.Map_Add` _ingredients _ingredient (+ _value Number))
    (else
      (`BlueprintMapLibrary.Map_Add` _ingredients _ingredient Number)))
  (`self.OnUpdateIngredient` (`self.Ingredients`)))

(fn `AddWeapon`
  (params (Weapon :type "/Game/05_BP/01_Player/DataAssets/Inventory/DA_Weapon Object Reference (by ref)"))
  (`KismetArrayLibrary.Array_Add` (`self.Weapons`) Weapon)
  (`self.OnUpdateWeapons` (`self.Weapons`)))

(fn `EquipBuff`
  (params (Buff :type "/Game/05_BP/01_Player/DataAssets/Inventory/Da_Buff Object Reference") (Slot :type Integer))
  (switch `int` Slot
    (:`1`
      (set `self.BuffSlot1` Buff))
    (:`2`
      (set `self.BuffSlot2` Buff))
    (:`3`
      (set `self.BuffSlot3` Buff)))
  (`self.OnUpdatedBuffs` (`self.Buffs`) (`self.BuffSlot1`) (`self.BuffSlot2`) (`self.BuffSlot3`)))

(fn `GetBuffNumber`
  (params (Buff :type "/Game/05_BP/01_Player/DataAssets/Inventory/Da_Buff Object Reference (by ref)"))
  (returns (Number :type Integer))
  (bind (_value _returnvalue) (`BlueprintMapLibrary.Map_Find` (`self.Buffs`) Buff))
  (return (`KismetMathLibrary.SelectInt` _value 0 _returnvalue)))

(fn `GetIngredientNumber`
  (params (Ingredient :type "/Game/05_BP/01_Player/DataAssets/Inventory/DA_Item Object Reference (by ref)"))
  (returns (Number :type Integer))
  (bind (_value _returnvalue) (`BlueprintMapLibrary.Map_Find` (`self.Ingredients`) Ingredient))
  (return (`KismetMathLibrary.SelectInt` _value 0 _returnvalue)))

(fn `HasWeapon`
  (params (Weapon :type "/Game/05_BP/01_Player/DataAssets/Inventory/DA_Weapon Object Reference (by ref)"))
  (returns (ReturnValue :type Boolean))
  (return (!= (`KismetArrayLibrary.Array_Find` (`self.Weapons`) Weapon) -1)))

(fn `RemoveBuff`
  (params (Buff :type "/Game/05_BP/01_Player/DataAssets/Inventory/Da_Buff Object Reference (by ref)") (Number :type Integer :default 1))
  (bind (_value _returnvalue) (`BlueprintMapLibrary.Map_Find` (`self.Buffs`) Buff))
  (if _returnvalue
    (`BlueprintMapLibrary.Map_Add` (`self.Buffs`) (`local.Buff`) (- _value Number))
    (`self.OnUpdatedBuffs` (`self.Buffs`) (`self.BuffSlot1`) (`self.BuffSlot2`) (`self.BuffSlot3`))))

(fn `RemoveIngredient`
  (params (Ingredient :type "/Game/05_BP/01_Player/DataAssets/Inventory/DA_Item Object Reference (by ref)") (Number :type Integer :default 1))
  (bind (_value _returnvalue) (`BlueprintMapLibrary.Map_Find` (`self.Ingredients`) Ingredient))
  (if _returnvalue
    (`BlueprintMapLibrary.Map_Add` (`self.Ingredients`) (`local.Ingredient`) (- _value Number))
    (`self.OnUpdateIngredient` (`self.Ingredients`))))

(fn `RemoveWeapon`
  (params (Weapon :type "/Game/05_BP/01_Player/DataAssets/Inventory/DA_Weapon Object Reference (by ref)"))
  (if (== (`KismetArrayLibrary.Array_Find` (`self.Weapons`) Weapon) -1)
    (`KismetArrayLibrary.Array_RemoveItem` (`self.Weapons`) (`local.Weapon`))
    (`self.OnUpdateWeapons` (`self.Weapons`))))