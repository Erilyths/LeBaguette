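; Player attack component for the Baker day character, handling melee and ranged attacks from the equipped weapons' data.
; Holding an input runs a looping timer that retries the attack, gated by cooldowns, with combo steps that reset at the end or after a delay.
; Melee damages actors in an oriented box overlap, with debug drawing left on.
; Ranged spawns and initializes bullets along the owner's forward vector, reloading on an empty magazine.
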(event `self.ReceiveBeginPlay`
  (bind _asbp_game_mode_day (cast `/Game/05_BP/05_GameMode/BP_GameModeDay` (`GameplayStatics.GetGameMode`)))
  (set `self.GameMode` _asbp_game_mode_day)
  (bind _asbp_baker_day (cast `/Game/05_BP/01_Player/BP_BakerDay` (`self.GetOwner`)))
  (set `self.Character` _asbp_baker_day)
  (set `self.CurrentBullets` (`/Game/05_BP/01_Player/DataAssets/Inventory/DA_RangeWeapon.MagSize` (`self.EquippedRange`))))

(event `EnhancedInput|/Game/05_BP/03_Input/Actions/IA_AttackMelee`
  (params (ActionValue :type Boolean) (ElapsedSeconds :type "Float (double-precision)") (TriggeredSeconds :type "Float (double-precision)") (InputAction :type "InputAction Object Reference" :default "/Game/05_BP/03_Input/Actions/IA_AttackMelee.IA_AttackMelee"))
  (bind _meleetimerhandle (`self.MeleeTimerHandle`))
  ;[0.6146 0.1387 0.08322 0.5] Melee
  (:`Started`
    (bind _returnvalue (`KismetSystemLibrary.K2_SetTimerDelegate` (delegate `Melee`) 0.1 true))
    (set `self.MeleeTimerHandle` _returnvalue)
    (`self.Melee`))
  (:`Completed`
    (`KismetSystemLibrary.K2_PauseTimerHandle` _meleetimerhandle)
    (`KismetSystemLibrary.K2_ClearAndInvalidateTimerHandle` _meleetimerhandle)))

(event `Melee`
  ;[0.6146 0.1387 0.08322 0.5] Melee
  (if (not (`self.MeleeOnCooldown`))
    (`self.Melee_Main`)
    (`|PlayMontage` (`Character.Mesh` (`GameplayStatics.GetPlayerCharacter` 0)) "/Game/08_Anim/AnimManny/Montage_Sword_Slash.Montage_Sword_Slash"
      (:`then`
        (`self.Melee_Delays`)))))

(event `Melee_Main`
  ;[0.6146 0.1387 0.08322 0.5] Melee
  (`self.CheckCubeCollider` (`|GetArrayItem` (`/Game/05_BP/01_Player/DataAssets/Inventory/DA_MeleeWeapon.Combos` (`self.EquippedMelee`)) (`self.MeleeCurrentCombo`)))
  (set `self.MeleeOnCombo` true)
  (set `self.MeleeOnCooldown` true)
  (if (< (`self.MeleeCurrentCombo`) (- (`KismetArrayLibrary.Array_Length` (`/Game/05_BP/01_Player/DataAssets/Inventory/DA_MeleeWeapon.Combos` (`self.EquippedMelee`))) 1))
    (`/Engine/EditorBlueprintResources/StandardMacros.IncrementInt` (`self.MeleeCurrentCombo`))
    (else
      (set `self.MeleeCurrentCombo` 0)
      (set `self.MeleeOnCombo` false))))

(event `Melee_Delays`
  ;[0.6146 0.1387 0.08322 0.5] Melee
  (`|ExecutionSequence`
    (:`then_0`
      (`KismetSystemLibrary.Delay` (* (`/Game/05_BP/01_Player/DataAssets/Inventory/DA_Weapon.AttackRate` (`self.EquippedMelee`)) (`self.AttackRateModifier`)))
      (set `self.MeleeOnCooldown` false))
    (:`then_1`
      (`KismetSystemLibrary.RetriggerableDelay` (`self.ComboLasting`))
      (set `self.MeleeCurrentCombo` 0)
      (set `self.MeleeOnCombo` false))))

(event `EnhancedInput|/Game/05_BP/03_Input/Actions/IA_AttackRange`
  (params (ActionValue :type Boolean) (ElapsedSeconds :type "Float (double-precision)") (TriggeredSeconds :type "Float (double-precision)") (InputAction :type "InputAction Object Reference" :default "/Game/05_BP/03_Input/Actions/IA_AttackRange.IA_AttackRange"))
  (bind _shoottimerhandle (`self.ShootTimerHandle`))
  ;[0.05604 0.15 0.02288 0.5] Shoot
  (:`Started`
    (bind _returnvalue (`KismetSystemLibrary.K2_SetTimerDelegate` (delegate `Shoot`) 0.1 true))
    (set `self.ShootTimerHandle` _returnvalue)
    (`self.Shoot`))
  (:`Completed`
    (`KismetSystemLibrary.K2_PauseTimerHandle` _shoottimerhandle)
    (`KismetSystemLibrary.K2_ClearAndInvalidateTimerHandle` _shoottimerhandle)))

(event `Shoot`
  ;[0.05604 0.15 0.02288 0.5] Shoot
  (if (== (`self.CurrentBullets`) 0)
    (if (not (`self.OnReload`))
      (`self.Shoot_Reload`))
    (elif (`KismetMathLibrary.BooleanNOR` (`self.RangeOnCooldown`) (`self.OnReload`))
      (`self.Shoot_Main`)
      (`self.Shoot_Delays`))))

(event `Shoot_Reload`
  (bind _equippedrange (`self.EquippedRange`))
  ;[0.05604 0.15 0.02288 0.5] Shoot
  (`KismetSystemLibrary.Delay` (`/Game/05_BP/01_Player/DataAssets/Inventory/DA_RangeWeapon.ReloadTime` _equippedrange))
  (set `self.CurrentBullets` (`/Game/05_BP/01_Player/DataAssets/Inventory/DA_RangeWeapon.MagSize` _equippedrange)))

(event `Shoot_Main`
  ;[0.05604 0.15 0.02288 0.5] Shoot
  (`self.SpawnBullet` (`|GetArrayItem` (`/Game/05_BP/01_Player/DataAssets/Inventory/DA_RangeWeapon.Combos` (`self.EquippedRange`)) (`self.RangeCurrentCombo`)))
  (set `self.RangeOnCombo` true)
  (set `self.RangeOnCooldown` true)
  (`/Engine/EditorBlueprintResources/StandardMacros.DecrementInt` (`self.CurrentBullets`)
    (:`  `
      (if (< (`self.RangeCurrentCombo`) (- (`KismetArrayLibrary.Array_Length` (`/Game/05_BP/01_Player/DataAssets/Inventory/DA_RangeWeapon.Combos` (`self.EquippedRange`))) 1))
        (`/Engine/EditorBlueprintResources/StandardMacros.IncrementInt` (`self.RangeCurrentCombo`))
        (else
          (set `self.RangeCurrentCombo` 0)
          (set `self.RangeOnCombo` false))))))

(event `Shoot_Delays`
  ;[0.05604 0.15 0.02288 0.5] Shoot
  (`|ExecutionSequence`
    (:`then_0`
      (`KismetSystemLibrary.Delay` (* (`/Game/05_BP/01_Player/DataAssets/Inventory/DA_Weapon.AttackRate` (`self.EquippedRange`)) (`self.AttackRateModifier`)))
      (set `self.RangeOnCooldown` false))
    (:`then_1`
      (`KismetSystemLibrary.Delay` (`self.ComboLasting`))
      (set `self.RangeCurrentCombo` 0)
      (set `self.RangeOnCombo` false))))

(fn `CheckCubeCollider`
  (params (AttackInfo :type "/Game/05_BP/01_Player/Struct/Struct_AttackZone Structure"))
  (bind _returnvalue (`self.GetOwner`))
  (bind ((`Extent_2_4D167D20404FA9C16E2F799EE664D48A` _extent) (`RelativePos_4_7651D177484024F884D39EA2289DBA82` _relativepos)) (break `/Game/05_BP/01_Player/Struct/Struct_AttackZone` (`local.AttackInfo`)))
  (bind _returnvalue_2 (`KismetMathLibrary.MakeRotator` (.roll (`Actor.K2_GetActorRotation` _returnvalue)) (.pitch (`Actor.K2_GetActorRotation` _returnvalue)) (+ (.yaw (`Actor.K2_GetActorRotation` _returnvalue)) 90.0)))
  (bind _returnvalue_3 (+ (`Actor.K2_GetActorLocation` _returnvalue) (* (`Actor.GetActorRightVector` _returnvalue) (.x _relativepos)) (* (`Actor.GetActorForwardVector` _returnvalue) (.y _relativepos))))
  (`KismetSystemLibrary.DrawDebugBox` _returnvalue_3 _extent (struct :`R` 1.0 :`G` 0.550446 :`B` 0.145359 :`A` 1.0) _returnvalue_2 5.0 5.0)
  (bind _outactors (`KismetSystemLibrary.BoxOverlapActorsWithOrientation` _returnvalue_3 _extent _returnvalue_2 (`|MakeArray` "ObjectTypeQuery1" "ObjectTypeQuery2" "ObjectTypeQuery3" :!type "EObjectTypeQuery Enum") null (`|MakeArray` (`self.GetOwner`))))
  (for _array_element _outactors
    (`GameplayStatics.ApplyDamage` _array_element (* (`.DamagesMultiplier_8_74161A9D4DF942C008CE7E9CAB2453B2` (break `/Game/05_BP/01_Player/Struct/Struct_AttackZone` (`local.AttackInfo`))) (`self.DamageBonus`) (`/Game/05_BP/01_Player/DataAssets/Inventory/DA_Weapon.BaseDamage` (`self.EquippedMelee`))))))

(fn `EquipMelee`
  (params (Melee :type "/Game/05_BP/01_Player/DataAssets/Inventory/DA_MeleeWeapon Object Reference"))
  (set `self.EquippedMelee` Melee))

(fn `EquipRange`
  (params (Range :type "/Game/05_BP/01_Player/DataAssets/Inventory/DA_RangeWeapon Object Reference"))
  (bind _output_get (set `self.EquippedRange` Range))
  (set `self.CurrentBullets` (`/Game/05_BP/01_Player/DataAssets/Inventory/DA_RangeWeapon.MagSize` _output_get)))

(fn `SpawnBullet`
  (params (BulletInfos :type "/Game/05_BP/01_Player/Struct/Struct_Bullet Structure"))
  (bind _returnvalue (`self.GetOwner`))
  (bind (_bullet _damagemultiplier) (break `/Game/05_BP/01_Player/Struct/Struct_Bullet` (`local.BulletInfos`)))
  (bind (_returnvalue_location _returnvalue_rotation) (`KismetMathLibrary.BreakTransform` (`Actor.GetTransform` _returnvalue)))
  (bind _returnvalue_2 (`|SpawnActorFromClass` _bullet (`KismetMathLibrary.MakeTransform` (+ (* (`Actor.GetActorForwardVector` _returnvalue) 10.0) _returnvalue_location) _returnvalue_rotation) "AlwaysSpawn" "MultiplyWithRoot" null null))
  (`/Game/05_BP/01_Player/BP_Bullet.Init` _returnvalue_2 (* (`self.DamageBonus`) _damagemultiplier (`/Game/05_BP/01_Player/DataAssets/Inventory/DA_Weapon.BaseDamage` (`self.EquippedRange`))) (`Actor.GetActorForwardVector` _returnvalue)))