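; Actor component that lets the cooking-game player, BP_BakerDay, drop a carried item.
; The carried item is stored as a class: DropItem, triggered by the T key, clears the owner's Item mesh and spawns that class at the owner's location.
; It then empties GrabbedItem but leaves HasItem unchanged; the F key prints the held class name for debugging.
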(event `Key|T`
  (params (Key :type "Key Structure"))
  (:`Pressed`
    (`self.Drop Item`)))

(event `Drop Item`
  (if (`self.has item`)
    (`self.GrabbedItem`
      (:`then`
        (`StaticMeshComponent.SetStaticMesh` (`/Game/leBaguette/Joa/BP_BakerDay.Item` (cast `/Game/leBaguette/Joa/BP_BakerDay` (`self.GetOwner`) :!pure true)) null)
        (`|SpawnActorFromClass` (`self.GrabbedItem`) (`KismetMathLibrary.MakeTransform` (`Actor.K2_GetActorLocation` (`self.GetOwner`))) "Undefined" "MultiplyWithRoot" null null)
        (set `self.GrabbedItem` null))
      (:`else`))))

(event `Key|F`
  (params (Key :type "Key Structure"))
  ;[0.15 0.005174 0.005604 0.5] Debug grabbed item
  (:`Pressed`
    (`KismetSystemLibrary.PrintString` (`KismetSystemLibrary.GetClassDisplayName` (`self.GrabbedItem`)))))