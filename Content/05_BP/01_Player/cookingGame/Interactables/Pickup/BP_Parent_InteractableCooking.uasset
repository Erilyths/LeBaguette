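; Parent Blueprint for pickup interactables in the cooking game, letting the baker player (BP_BakerDay) carry an item.
; On Interact by player 0 with empty hands, it copies its mesh, material and scale onto the character's Item component.
; It then records the grabbed item in the character's ACBPCarryObject component and destroys itself, so the carried item is a visual swap rather than an attachment.
; Interaction getters supply the "to carry" prompt, interaction type and timing values.
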(event `self.ReceiveBeginPlay`
  (bind _asbp_baker_day (cast `/Game/05_BP/01_Player/BP_BakerDay` (`GameplayStatics.GetPlayerCharacter` 0)))
  (set `self.CharaRef` _asbp_baker_day))

(event `/Game/05_BP/01_Player/InteractionSystem/BPI_Interactable.Interact`
  (params (Interactor :type "Actor Object Reference"))
  (bind _chararef (`self.CharaRef`))
  (bind _item (`/Game/05_BP/01_Player/BP_BakerDay.Item` _chararef))
  (`/Game/05_BP/01_Player/cookingGame/AC_BP_CarryObject.GrabbedItem` (`/Game/05_BP/01_Player/BP_BakerDay.AC_BP_CarryObject` (`self.CharaRef`))
    (:`then`)
    (:`else`
      (if (== Interactor (`GameplayStatics.GetPlayerCharacter` 0))
        (set `/Game/05_BP/01_Player/cookingGame/AC_BP_CarryObject.has item` true (`/Game/05_BP/01_Player/BP_BakerDay.AC_BP_CarryObject` _chararef))
        (set `self.Item` _item)
        (`PrimitiveComponent.SetMaterial` _item 0 (`self.Material`))
        (`StaticMeshComponent.SetStaticMesh` _item (`StaticMeshComponent.StaticMesh` (`self.StaticMesh`)))
        (`SceneComponent.K2_SetRelativeTransform` _item (`KismetMathLibrary.MakeTransform` (0.0 0.0 0.0) (struct) (`self.Scale`)) false false)
        (set `/Game/05_BP/01_Player/cookingGame/AC_BP_CarryObject.GrabbedItem` (`self.Grabbed Item`) (`/Game/05_BP/01_Player/BP_BakerDay.AC_BP_CarryObject` (`self.CharaRef`)))
        (`self.K2_DestroyActor`)))))

(fn `GetHoldDuration`
  (returns (Duration :type "Float (double-precision)"))
  (return 2.0))

(fn `GetInteractionLocation`
  (returns (`Location ` :type "Vector Structure"))
  (return (0.0 0.0 0.0)))

(fn `GetInteractionPrompt`
  (returns (Value :type Text))
  (return "to carry"))

(fn `GetInteractionType`
  (returns (Type :type "/Game/05_BP/01_Player/InteractionSystem/E_InteractionTypes Enum"))
  (return "NewEnumerator0"))

(fn `GetTapCount`
  (returns (Value :type Integer))
  (return 0))

(fn `UserConstructionScript`)