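; Base loot item Blueprint for ingredient pickups that the player collects on contact.
; On BeginPlay it applies the mesh and material from its DAItem data asset, or prints a debug string if unset, then launches the mesh with a randomized upward impulse.
; When the player character overlaps the sphere collider, it moves the mesh toward the player, adds one ingredient to AC_BP_Inventory and destroys itself.
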(event `self.ReceiveBeginPlay`
  (bind _da_item (`self.DA Item`))
  (bind _mesh (`self.Mesh`))
  (bind _mesh_2 (`/Game/leBaguette/Joa/DataAssets/Inventory/DA_Item.Mesh` _da_item))
  (`/Engine/EditorBlueprintResources/StandardMacros.IsValid` _da_item
    (:`Is Valid`
      (`StaticMeshComponent.SetStaticMesh` _mesh _mesh_2)
      (`PrimitiveComponent.SetMaterial` _mesh 0 (`StaticMesh.GetMaterial` _mesh_2 0)))
    (:`Is Not Valid`
      (`KismetSystemLibrary.PrintString` "CACA" true true (struct :`R` 1.0 :`G` 0.009247 :`B` 4e-05 :`A` 1.0))))
  (`PrimitiveComponent.AddImpulse` (`self.Mesh`) (* (`KismetMathLibrary.MakeVector` (`KismetMathLibrary.RandomFloatInRange` -1.0 1.0) (`KismetMathLibrary.RandomFloatInRange` -1.0 1.0) 1.0) 5000.0) "None" false))

(event `self.SphereCollider.OnComponentBeginOverlap`
  (params (OverlappedComponent :type "PrimitiveComponent Object Reference") (OtherActor :type "Actor Object Reference") (OtherComp :type "PrimitiveComponent Object Reference") (OtherBodyIndex :type Integer) (bFromSweep :type Boolean) (SweepResult :type "HitResult Structure (by ref)"))
  (bind _returnvalue (`GameplayStatics.GetPlayerCharacter` 0))
  (if (== OtherActor _returnvalue)
    (`KismetSystemLibrary.MoveComponentTo` (`self.Mesh`) (`self.K2_GetActorLocation` _returnvalue))
    (`/Game/leBaguette/Joa/ActorComponent/AC_BP_Inventory.AddIngredient` (`self.GetComponentByClass` (`GameplayStatics.GetPlayerCharacter` 0) "/Game/leBaguette/Joa/ActorComponent/AC_BP_Inventory.AC_BP_Inventory_C") (`self.DA Item`) 1)
    (`KismetSystemLibrary.PrintString` (`KismetSystemLibrary.GetDisplayName` self))
    (`self.K2_DestroyActor`)))

(fn `UserConstructionScript`)