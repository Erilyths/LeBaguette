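; Loot actor component that picks an item by weighted rarity and spawns it at its owner's location.
; ChooseRarity sums the RarityMap weights, rolls within that total and subtracts weights until it lands on a key.
; BeginPlay rolls once, and SpawnItems passes that result as the data asset to every BP_Parent_Items it spawns.
; TestLoot tallies repeated rolls and prints the counts to check the distribution.
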(event `TestLoot`
  (bind _temp (`self.temp`))
  (for _ (range 1001)
    (bind _rarityoutput (`self.ChooseRarity`))
    (`BlueprintMapLibrary.Map_Add` _temp _rarityoutput (+ (`BlueprintMapLibrary.Map_Find` _temp _rarityoutput) 1)))
  (bind (_keypin _valuepin) (`|MapForEach` (`self.temp`))
    (:`then`
      (`KismetSystemLibrary.PrintString` (`KismetStringLibrary.Concat_StrStr` "" " / " (`KismetStringLibrary.Conv_IntToString` _valuepin)) true true (struct :`G` 0.66 :`B` 1.0 :`A` 1.0) 60.0))))

(event `self.ReceiveBeginPlay`
  (bind _rarityoutput (`self.ChooseRarity`))
  (set `self.ItemRarity` _rarityoutput))

(event `SpawnItems`
  (for _ (range (`self.NumberOfItems`))
    (`|SpawnActorFromClass` "/Game/05_BP/01_Player/LootSystem/LootItems/BP_Parent_Items.BP_Parent_Items_C" (`KismetMathLibrary.MakeTransform` (`Actor.K2_GetActorLocation` (`self.GetOwner`))) "AdjustIfPossibleButAlwaysSpawn" "MultiplyWithRoot" null (`self.ItemRarity`) null)))

(fn `ChooseRarity`
  (returns (RarityOutput :type "/Game/leBaguette/Joa/DataAssets/Inventory/DA_Item Object Reference"))
  (locals (SumOfRarities :type "Float (double-precision)") (LootRoll :type "Float (double-precision)" :default 0.0) (RarityOut :type "/Game/leBaguette/Joa/DataAssets/Inventory/DA_Item Object Reference"))
  (bind _raritymap (`self.RarityMap`))
  (bind _raritymap_2 (`self.RarityMap`))
  ; SumOfRarity
  (bind _keys (`BlueprintMapLibrary.Map_Keys` _raritymap))
  (for _array_element _keys
    (set `local.SumOfRarities` (+ (`BlueprintMapLibrary.Map_Find` _raritymap _array_element) (`local.SumOfRarities`))))
  ; LootRoll
  (set `local.LootRoll` (`KismetMathLibrary.RandomFloatInRange` 0.0 (`local.SumOfRarities`)))
  ; Debug
  (`KismetSystemLibrary.PrintString` (`KismetStringLibrary.Conv_DoubleToString` (`local.LootRoll`)) true true (struct :`R` 1.0 :`B` 0.125723 :`A` 1.0))
  (`KismetSystemLibrary.PrintString` (`KismetStringLibrary.Conv_DoubleToString` (`local.SumOfRarities`)))
  (bind _keys_2 (`BlueprintMapLibrary.Map_Keys` _raritymap_2))
  (for _array_element_2 _keys_2
    (bind _value (`BlueprintMapLibrary.Map_Find` _raritymap_2 _array_element_2))
    (if (>= _value (`local.LootRoll`))
      (set `local.RarityOut` _array_element_2)
      (break)
      (else
        (set `local.LootRoll` (- (`local.LootRoll`) _value)))))
  (`KismetSystemLibrary.PrintString` "Hello" true true (struct :`R` 1.0 :`B` 0.906368 :`A` 1.0))
  (return (`local.RarityOut`)))