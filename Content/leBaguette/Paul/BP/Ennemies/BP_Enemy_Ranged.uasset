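; Ranged enemy Blueprint that spawns a gun at BeginPlay, attaches it to its hand socket and fights from a fixed ideal range.
; Attack plays a pistol fire montage; its notify line-traces from the weapon toward the AI controller's attack target and applies damage only if nothing blocks the trace.
; Montage completion or interruption signals attack end.
; Helper functions map movement states to walk speeds and report attack and defend radii.
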(event `self.ReceiveBeginPlay`
  (`parent.ReceiveBeginPlay`)
  (`self.EquipWeapon`))

(event `/Game/leBaguette/Paul/BP/Ennemies/AI/BPI_EnemyAI.EquipWeapon`
  (bind _returnvalue (`|SpawnActorFromClass` "/Game/leBaguette/Paul/Weapons/BP_Weapon_Gun.BP_Weapon_Gun_C" (`KismetMathLibrary.MakeTransform` (0.0 0.0 0.0)) "Undefined" "MultiplyWithRoot" null null))
  (bind _output_get (set `self.WeaponActor` _returnvalue))
  (`self.K2_AttachToComponent` _output_get (`self.Mesh`) "hand_r_sword_socket" "SnapToTarget" "SnapToTarget" "SnapToTarget" true)
  (set `self.isWieldingWeapon` true))

(event `/Game/leBaguette/Paul/BP/Ennemies/AI/BPI_EnemyAI.Attack`
  (bind _notifyname (`|PlayMontage` (`self.Mesh`) "/Game/Characters/Mannequins/Anims/Pistol/MM_Pistol_Fire_Montage.MM_Pistol_Fire_Montage")
    (:`OnCompleted`
      (`self.OnAttackEnd` :!label _label))
    (:`OnInterrupted`
      (goto _label))
    (:`OnNotifyBegin`
      (switch `name` _notifyname
        (:`Fire`
          (bind _asaic_ennemy_base (cast `/Game/leBaguette/Paul/BP/Ennemies/AI/AIC_Ennemy_Base` (`AIBlueprintHelperLibrary.GetAIController` self)))
          (bind _attack_target (`/Game/leBaguette/Paul/BP/Ennemies/AI/AIC_Ennemy_Base.Attack Target` _asaic_ennemy_base)
            (:`then`
              (bind (_outhit _returnvalue) (`KismetSystemLibrary.LineTraceSingle` :`Start` (+ (`self.K2_GetActorLocation` (`self.WeaponActor`)) (0.0 0.0 100.0)) :`End` (+ (`self.K2_GetActorLocation` _attack_target) (0.0 0.0 50.0)) :`TraceChannel` "TraceTypeQuery1" :`DrawDebugType` "ForDuration"))
              (if (not _returnvalue)
                (`GameplayStatics.ApplyDamage` _attack_target 20.0)))
            (:`else`)))))))

(fn `Get Ideal Range`
  (returns (AttackRadius :type "Float (double-precision)") (DefendRadius :type "Float (double-precision)"))
  (return 600.0 600.0))

(fn `SetMovementSpeed`
  (params (Speed :type "/Game/leBaguette/Paul/BP/Ennemies/AI/Enum/E_MovementSpeed Enum" :default "NewEnumerator0"))
  (returns (SpeedValue :type "Float (double-precision)"))
  (bind _output_get (set `CharacterMovementComponent.MaxWalkSpeed` (select `/Game/leBaguette/Paul/BP/Ennemies/AI/Enum/E_MovementSpeed` Speed :`NewEnumerator1` 200.0 :`NewEnumerator2` 300.0 :`NewEnumerator3` 500.0 :!type "Float (single-precision)") (`self.CharacterMovement`)))
  (return _output_get))

(fn `UserConstructionScript`
  (`parent.UserConstructionScript`))