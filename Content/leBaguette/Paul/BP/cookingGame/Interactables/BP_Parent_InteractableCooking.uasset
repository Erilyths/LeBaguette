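; Parent Blueprint for cooking-game items that the player picks up to carry, using a "to carry" interaction prompt.
; On Interact by player 0 with no valid GrabbedItem, it copies its material, mesh and scale onto the BP_Chara Item component.
; It then sets the character's GrabbedItem and destroys itself, so the carried object is a visual stand-in rather than the attached actor.
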(event `self.ReceiveBeginPlay`
  (bind _asbp_chara (cast `/Game/leBaguette/Paul/BP/BP_Chara` (`GameplayStatics.GetPlayerCharacter` 0)))
  (set `self.CharaRef` _asbp_chara))

(event `/Game/leBaguette/Paul/BP/InteractionSystem/BPI_Interactable.Interact`
  (params (Interactor :type "Actor Object Reference"))
  (bind _item (`/Game/leBaguette/Paul/BP/BP_Chara.Item` (`self.CharaRef`)))
  (`/Game/leBaguette/Paul/BP/BP_Chara.GrabbedItem` (`self.CharaRef`)
    (:`then`)
    (:`else`
      (if (== Interactor (`GameplayStatics.GetPlayerCharacter` 0))
        (set `self.Item` _item)
        (`PrimitiveComponent.SetMaterial` _item 0 (`self.Material`))
        (`StaticMeshComponent.SetStaticMesh` _item (`StaticMeshComponent.StaticMesh` (`self.StaticMesh`)))
        (`SceneComponent.K2_SetRelativeTransform` _item (`KismetMathLibrary.MakeTransform` (0.0 0.0 0.0) (struct) (`self.Scale`)) false false)
        (set `/Game/leBaguette/Paul/BP/BP_Chara.GrabbedItem` (`self.Grabbed Item`) (`self.CharaRef`))
        (`self.K2_DestroyActor`)))))

(fn `GetHoldDuration`
  (returns (Duration :type "Float (double-precision)"))
  (return 2.0))

(fn `GetInteractionLocation`
  (returns (`Location ` :type "Vector Structure"))
  (return (0.0 0.0 0.0)))

(fn `GetInteractionPrompt`
  (returns (Value :type Text))
  (return "to carry"))

(fn `GetInteractionType`
  (returns (Type :type "/Game/leBaguette/Paul/BP/InteractionSystem/E_InteractionTypes Enum"))
  (return "NewEnumerator0"))

(fn `GetTapCount`
  (returns (Value :type Integer))
  (return 0))

(fn `UserConstructionScript`)