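; Parent cutting board furniture for the cooking game, an interactable where the player places a carried item and then cuts it.
; With the board empty, interacting takes the BP_BakerDay's grabbed item, clears the hand mesh and spawns it on the board without physics.
; The interaction type changes once an item is placed.
; Cutting is a stub that prints and destroys the item, leaving HasItemOnIt set.
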(event `self.ReceiveBeginPlay`
  (bind _asbp_baker_day (cast `/Game/leBaguette/Joa/BP_BakerDay` (`GameplayStatics.GetPlayerCharacter` 0)))
  (set `self.Chara ref 2` _asbp_baker_day))

(event `/Game/leBaguette/Paul/BP/InteractionSystem/BPI_Interactable.Interact`
  (params (Interactor :type "Actor Object Reference"))
  (bind _chara_ref_2 (`self.Chara ref 2`))
  (bind _ac_bp_carryobject (`/Game/leBaguette/Joa/BP_BakerDay.AC_BP_CarryObject` _chara_ref_2))
  (if (`self.hasItemOnIt`)
    (`self.Cut`)
    (elif (== Interactor (`GameplayStatics.GetPlayerCharacter` 0))
      (set `/Game/leBaguette/Paul/BP/cookingGame/AC_BP_CarryObject.has item` false _ac_bp_carryobject)
      (bind _grabbeditem (`/Game/leBaguette/Paul/BP/cookingGame/AC_BP_CarryObject.GrabbedItem` _ac_bp_carryobject)
        (:`then`
          (`StaticMeshComponent.SetStaticMesh` (`/Game/leBaguette/Joa/BP_BakerDay.Item` _chara_ref_2) null)
          (bind _returnvalue (`|SpawnActorFromClass` _grabbeditem (`KismetMathLibrary.MakeTransform` (`SceneComponent.K2_GetComponentLocation` (`self.Item`))) "Undefined" "MultiplyWithRoot" null null))
          (bind _output_get (set `self.ItemOnPlanch` _returnvalue))
          (`PrimitiveComponent.SetSimulatePhysics` (`/Game/leBaguette/Paul/BP/cookingGame/Interactables/Pickup/BP_Parent_InteractableCooking.StaticMesh` _output_get) false)
          (set `self.hasItemOnIt` true))
        (:`else`)))))

(event `Cut`
  (`KismetSystemLibrary.PrintString` "cut")
  (`self.K2_DestroyActor` (`self.ItemOnPlanch`)))

(fn `GetHoldDuration`
  (returns (Duration :type "Float (double-precision)"))
  (return 1.0))

(fn `GetInteractionLocation`
  (returns (`Location ` :type "Vector Structure"))
  (return (0.0 0.0 0.0)))

(fn `GetInteractionPrompt`
  (returns (Value :type Text))
  (return "To Cut"))

(fn `GetInteractionType`
  (returns (Type :type "/Game/leBaguette/Paul/BP/InteractionSystem/E_InteractionTypes Enum"))
  (if (`self.hasItemOnIt`)
    (return "NewEnumerator1")
    (else
      (return "NewEnumerator0"))))

(fn `GetTapCount`
  (returns (Value :type Integer))
  (return 0))

(fn `UserConstructionScript`)