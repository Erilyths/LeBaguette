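; Tomato interactable for the cooking game, a child Blueprint of a parent that supplies the base behavior.
; On BeginPlay it runs the parent logic, then sets its scale and material and records its own class as the grabbed item.
; It overrides the interaction queries to return the first interaction type with zero hold duration.
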(event `self.ReceiveBeginPlay`
  (`parent.ReceiveBeginPlay`)
  (set `self.Scale` (`self.Scale`))
  (set `self.Material` "/Game/leBaguette/Paul/BP/LootSystem/LootItems/Materials/MI_7Unreal.MI_7Unreal")
  (set `self.Grabbed Item` (`GameplayStatics.GetObjectClass` self)))

(fn `GetHoldDuration`
  (returns (Duration :type "Float (double-precision)"))
  (return 0.0))

(fn `GetInteractionType`
  (returns (Type :type "/Game/leBaguette/Paul/BP/InteractionSystem/E_InteractionTypes Enum"))
  (return "NewEnumerator0"))

(fn `UserConstructionScript`
  (`parent.UserConstructionScript`))