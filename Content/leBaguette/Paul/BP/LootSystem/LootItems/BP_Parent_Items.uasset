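; BP_Parent_Items is a loot item actor, named as a parent class for items, that pops out when spawned and is picked up on touch.
; On BeginPlay its mesh gets an upward impulse with a random horizontal direction.
; When the sphere collider overlaps player character 0, it prints its own name and destroys itself, with no inventory or reward logic.
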(event `self.ReceiveBeginPlay`
  (`PrimitiveComponent.AddImpulse` (`self.Mesh`) (* (`KismetMathLibrary.MakeVector` (`KismetMathLibrary.RandomFloatInRange` -1.0 1.0) (`KismetMathLibrary.RandomFloatInRange` -1.0 1.0) 1.0) 5000.0) "None" false))

(event `self.SphereCollider.OnComponentBeginOverlap`
  (params (OverlappedComponent :type "PrimitiveComponent Object Reference") (OtherActor :type "Actor Object Reference") (OtherComp :type "PrimitiveComponent Object Reference") (OtherBodyIndex :type Integer) (bFromSweep :type Boolean) (SweepResult :type "HitResult Structure (by ref)"))
  (if (== OtherActor (`GameplayStatics.GetPlayerCharacter` 0))
    (`KismetSystemLibrary.PrintString` (`KismetSystemLibrary.GetDisplayName` self))
    (`self.K2_DestroyActor`)))

(fn `UserConstructionScript`)