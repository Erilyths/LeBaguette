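; Loot actor component that spawns item actors of a randomly rolled rarity at its owner's location on BeginPlay.
; ChooseRarity does a weighted roll over RarityMap, summing the weights and subtracting each from the roll until one covers it, with debug prints.
; SpawnItems maps that single rolled rarity to one of seven child Blueprint classes, Poor through Unreal, and spawns NumberOfItems copies of it.
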(event `self.ReceiveBeginPlay`
  (bind _rarityoutput (`self.ChooseRarity`))
  (set `self.ItemRarity` _rarityoutput)
  (`self.SpawnItems`))

(event `SpawnItems`
  (for _ (range (`self.NumberOfItems`))
    (`|SpawnActorFromClass` (select `/Game/leBaguette/Paul/BP/LootSystem/E_LootRarity` (`self.ItemRarity`) :`NewEnumerator0` "/Game/leBaguette/Paul/BP/LootSystem/LootItems/BP_Child_1Poor.BP_Child_1Poor_C" :`NewEnumerator1` "/Game/leBaguette/Paul/BP/LootSystem/LootItems/BP_Child_2Common.BP_Child_2Common_C" :`NewEnumerator2` "/Game/leBaguette/Paul/BP/LootSystem/LootItems/BP_Child_3Uncommon.BP_Child_3Uncommon_C" :`NewEnumerator3` "/Game/leBaguette/Paul/BP/LootSystem/LootItems/BP_Child_4Rare.BP_Child_4Rare_C" :`NewEnumerator4` "/Game/leBaguette/Paul/BP/LootSystem/LootItems/BP_Child_5Epic.BP_Child_5Epic_C" :`NewEnumerator5` "/Game/leBaguette/Paul/BP/LootSystem/LootItems/BP_Child_6Legendary.BP_Child_6Legendary_C" :`NewEnumerator6` "/Game/leBaguette/Paul/BP/LootSystem/LootItems/BP_Child_7Unreal.BP_Child_7Unreal_C" :!type "Actor Class Reference") (`KismetMathLibrary.MakeTransform` (`Actor.K2_GetActorLocation` (`self.GetOwner`))) "Undefined" "MultiplyWithRoot" null null)))

(fn `ChooseRarity`
  (returns (RarityOutput :type "/Game/leBaguette/Paul/BP/LootSystem/E_LootRarity Enum"))
  (locals (SumOfRarities :type "Float (double-precision)") (LootRoll :type "Float (double-precision)" :default 0.0) (RarityOut :type "/Game/leBaguette/Paul/BP/LootSystem/E_LootRarity Enum"))
  (bind _raritymap (`self.RarityMap`))
  (bind _rarityout (`local.RarityOut`))
  (bind _raritymap_2 (`self.RarityMap`))
  ; SumOfRarity
  (bind _keys (`BlueprintMapLibrary.Map_Keys` _raritymap))
  (for _array_element _keys
    (set `local.SumOfRarities` (+ (`BlueprintMapLibrary.Map_Find` _raritymap _array_element) (`local.SumOfRarities`))))
  ; LootRoll
  (set `local.LootRoll` (`KismetMathLibrary.RandomFloatInRange` 0.0 (`local.SumOfRarities`)))
  ; Debug
  (`KismetSystemLibrary.PrintString` (`KismetStringLibrary.Conv_DoubleToString` (`local.LootRoll`)) true true (struct :`R` 1.0 :`B` 0.125723 :`A` 1.0))
  (`KismetSystemLibrary.PrintString` (`KismetStringLibrary.Conv_DoubleToString` (`local.SumOfRarities`)))
  (bind _keys_2 (`BlueprintMapLibrary.Map_Keys` _raritymap_2))
  (for _array_element_2 _keys_2
    (bind _value (`BlueprintMapLibrary.Map_Find` _raritymap_2 _array_element_2))
    (if (>= _value (`local.LootRoll`))
      (set `local.RarityOut` _array_element_2)
      (break)
      (else
        (set `local.LootRoll` (- (`local.LootRoll`) _value)))))
  (`KismetSystemLibrary.PrintString` (`|GetEnumeratorNameAsString` _rarityout) true true (struct :`R` 1.0 :`B` 0.906368 :`A` 1.0))
  (return _rarityout))