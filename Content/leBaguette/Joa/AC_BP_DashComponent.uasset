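; Actor component that gives BP_BakerDay a charge-based dash on the IA_Jump input.
; A dash spends a charge and launches the baker horizontally along the capsule's forward vector, tuned by the baker's MetricsDataAsset.
; Chained Delays hold the dash state for its duration, then return a charge after a cooldown.
; Charge changes are pushed to the dash HUD through BP_GameModeDay.
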(event `self.ReceiveBeginPlay`
  (bind _asbp_baker_day (cast `/Game/leBaguette/Joa/BP_BakerDay` (`self.GetOwner`)))
  (set `self.BakerRef` _asbp_baker_day)
  (bind _output_get (set `self.DashCount` (`/Game/leBaguette/Joa/DataAssets/DA_BakerDayMetrics.MaxDashCount` (`/Game/leBaguette/Joa/BP_BakerDay.MetricsDataAsset` (`self.BakerRef`)))))
  (bind _asbp_game_mode_day (cast `/Game/leBaguette/Joa/BP_GameModeDay` (`GameplayStatics.GetGameMode`))
    (:`then`
      (bind _output_get_2 (set `self.Game Mode` _asbp_game_mode_day))
      (`/Game/leBaguette/Joa/BP_GameModeDay.UpdateDashHud` _output_get_2 _output_get))
    (:`CastFailed`
      (`KismetSystemLibrary.PrintString` "Failed to Cast Game Mode Day (maybe using baker day without gamemode day)" true true (struct :`R` 1.0 :`A` 1.0) 5.0))))

(event `EnhancedInput|/Game/leBaguette/Paul/Input/Actions/IA_Jump`
  (params (ActionValue :type Boolean) (ElapsedSeconds :type "Float (double-precision)") (TriggeredSeconds :type "Float (double-precision)") (InputAction :type "InputAction Object Reference" :default "/Game/leBaguette/Paul/Input/Actions/IA_Jump.IA_Jump"))
  (bind _bakerref (`self.BakerRef`))
  (bind _bakerref_2 (`self.BakerRef`))
  (bind _metricsdataasset (`/Game/leBaguette/Joa/BP_BakerDay.MetricsDataAsset` _bakerref))
  (bind (_returnvalue_x _returnvalue_y) (`KismetMathLibrary.BreakVector` (`KismetMathLibrary.GetForwardVector` (`SceneComponent.RelativeRotation` (`Character.CapsuleComponent` _bakerref)))))
  ; Dash
  (:`Triggered`
    (if (and (>= (`self.DashCount`) 1) (`/Game/leBaguette/Joa/BP_BakerDay.canDash` _bakerref))
      (bind _result (`/Engine/EditorBlueprintResources/StandardMacros.DecrementInt` (`self.DashCount`))
        (:`  `
          (`/Game/leBaguette/Joa/BP_GameModeDay.UpdateDashHud` (`self.Game Mode`) _result)
          (`Character.LaunchCharacter` _bakerref_2 (* (`KismetMathLibrary.MakeVector` _returnvalue_x _returnvalue_y) (`/Game/leBaguette/Joa/DataAssets/DA_BakerDayMetrics.DashPower` _metricsdataasset) 10.0) false false)
          (`/Game/leBaguette/Joa/BP_BakerDay.SwitchState` _bakerref_2 "NewEnumerator1")
          (`KismetSystemLibrary.Delay` (`/Game/leBaguette/Joa/DataAssets/DA_BakerDayMetrics.DashTime` _metricsdataasset))
          (`/Game/leBaguette/Joa/BP_BakerDay.SwitchState` _bakerref_2 "NewEnumerator0")
          (`KismetSystemLibrary.Delay` (`/Game/leBaguette/Joa/DataAssets/DA_BakerDayMetrics.DashCooldown` _metricsdataasset))
          (bind _result_2 (`/Engine/EditorBlueprintResources/StandardMacros.IncrementInt` (`self.DashCount`))
            (:`  `
              (`/Game/leBaguette/Joa/BP_GameModeDay.UpdateDashHud` (`self.Game Mode`) _result_2))))))))