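; BP_GameModeDay is a game mode that creates the HUD and gives the player a starting loadout.
; On BeginPlay it adds WBP_Hud to the viewport, then adds a bow and a sword data asset to BPInventorySystem and equips them as Range and Melee weapons.
; EquipWeapon routes by type to the inventory and refreshes the HUD's equipped weapons on success.
; UpdateDashHud forwards the dash count to the HUD.
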(event `self.ReceiveBeginPlay`
  (bind _returnvalue (`|GenericCreateObject` "/Game/leBaguette/Joa/WBP_Hud.WBP_Hud_C"))
  (bind _output_get (set `self.HudWidget` _returnvalue))
  (`UserWidget.AddToViewport` _output_get 0)
  (`self.SetupInventory`))

(fn `EquipWeapon`
  (params (Type :type "/Game/leBaguette/Joa/Struct/Enum_WeaponType Enum" :default "NewEnumerator0") (Index :type Integer))
  (returns (Equipped :type Boolean))
  (bind _bp_inventorysystem (`self.BP_InventorySystem`))
  (switch `/Game/leBaguette/Joa/Struct/Enum_WeaponType` Type
    (:`NewEnumerator0`
      (bind _equipped (`/Game/leBaguette/Joa/BP_InventorySystemComponent.EquipMelee` _bp_inventorysystem Index))
      (if _equipped
        _
        (else
          (return false))))
    (:`NewEnumerator1`
      (bind _equipped_2 (`/Game/leBaguette/Joa/BP_InventorySystemComponent.EquipRange` _bp_inventorysystem Index))
      (if _equipped_2
        _
        (else
          (return false)))))
  (`self.UpdateEquipedWeaponsHud`)
  (return true))

(fn `SetupInventory`
  (bind _bp_inventorysystem (`self.BP_InventorySystem`))
  (bind (_added _index) (`/Game/leBaguette/Joa/BP_InventorySystemComponent.AddWeapon` _bp_inventorysystem "/Game/leBaguette/Joa/Weapon/Weapons/DA_Bow01.DA_Bow01"))
  (if _added
    (`self.EquipWeapon` "NewEnumerator1" _index))
  (bind (_added_2 _index_2) (`/Game/leBaguette/Joa/BP_InventorySystemComponent.AddWeapon` _bp_inventorysystem "/Game/leBaguette/Joa/Weapon/Weapons/DA_Sword01.DA_Sword01"))
  (if _added_2
    (`self.EquipWeapon` "NewEnumerator0" _index_2)))

(fn `UpdateDashHud`
  (params (Count :type Integer))
  (`/Game/leBaguette/Joa/WBP_Hud.UpdateDash` (`self.HudWidget`) Count))

(fn `UpdateEquipedWeaponsHud`
  (bind _hudwidget (`self.HudWidget`))
  (bind _bp_inventorysystem (`self.BP_InventorySystem`))
  (bind _equippedmelee (`/Game/leBaguette/Joa/BP_InventorySystemComponent.EquippedMelee` _bp_inventorysystem))
  (bind _equippedrange (`/Game/leBaguette/Joa/BP_InventorySystemComponent.EquippedRange` _bp_inventorysystem))
  (`/Engine/EditorBlueprintResources/StandardMacros.IsValid` _equippedmelee
    (:`Is Valid`
      (`/Game/leBaguette/Joa/WBP_Hud.UpdateEquippedMelee` _hudwidget _equippedmelee))
    (:`Is Not Valid`
      _))
  (`/Engine/EditorBlueprintResources/StandardMacros.IsValid` _equippedrange
    (:`Is Valid`
      (`/Game/leBaguette/Joa/WBP_Hud.UpdateEquippedRange` _hudwidget _equippedrange))
    (:`Is Not Valid`
      _))
  (return))

(fn `UserConstructionScript`)