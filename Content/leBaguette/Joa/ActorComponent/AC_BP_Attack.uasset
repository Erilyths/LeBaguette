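; Attack component for the day-phase baker that handles melee and ranged combo attacks from Enhanced Input.
; Each attack reads the current combo step of the equipped weapon, advances it, and uses delays for a rate-scaled cooldown and combo reset.
; Melee runs a debug-drawn oriented box overlap and sends bonus-scaled damage through BPI_Attack.
; Ranged spawns the step's bullet along the owner's forward vector, initialized with damage and speed.
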(event `self.ReceiveBeginPlay`
  (bind _asbp_game_mode_day (cast `/Game/leBaguette/Joa/BP_GameModeDay` (`GameplayStatics.GetGameMode`)))
  (set `self.GameMode` _asbp_game_mode_day)
  (bind _asbp_baker_day (cast `/Game/leBaguette/Joa/BP_BakerDay` (`self.GetOwner`)))
  (set `self.Character` _asbp_baker_day))

(event `EnhancedInput|/Game/leBaguette/Paul/Input/Actions/IA_AttackMelee`
  (params (ActionValue :type Boolean) (ElapsedSeconds :type "Float (double-precision)") (TriggeredSeconds :type "Float (double-precision)") (InputAction :type "InputAction Object Reference" :default "/Game/leBaguette/Paul/Input/Actions/IA_AttackMelee.IA_AttackMelee"))
  (bind (_extent _relativepos _damagesmultiplier) (break `/Game/leBaguette/Joa/Struct/Struct_AttackZone` (`|GetArrayItem` (`/Game/leBaguette/Joa/DataAssets/Inventory/DA_MeleeWeapon.Combos` (`self.EquippedMelee`)) (`self.MeleeCurrentCombo`))))
  (:`Triggered`
    (if (not (`self.MeleeOnCooldown`))
      (`self.CheckCubeCollider` _extent _relativepos _damagesmultiplier)
      (set `self.MeleeOnCombo` true)
      (set `self.MeleeOnCooldown` true)
      (if (< (`self.MeleeCurrentCombo`) (- (`KismetArrayLibrary.Array_Length` (`/Game/leBaguette/Joa/DataAssets/Inventory/DA_MeleeWeapon.Combos` (`self.EquippedMelee`))) 1))
        (`/Engine/EditorBlueprintResources/StandardMacros.IncrementInt` (`self.MeleeCurrentCombo`)
          (:`  `
            _))
        (else
          (set `self.MeleeCurrentCombo` 0)
          (set `self.MeleeOnCombo` false)))
      (`|ExecutionSequence`
        (:`then_0`
          (`KismetSystemLibrary.Delay` (* (`/Game/leBaguette/Joa/DataAssets/Inventory/DA_Weapon.AttackRate` (`self.EquippedMelee`)) (`self.AttackRateModifier`)))
          (set `self.MeleeOnCooldown` false))
        (:`then_1`
          (`KismetSystemLibrary.RetriggerableDelay` (`self.ComboLasting`))
          (set `self.MeleeCurrentCombo` 0)
          (set `self.MeleeOnCombo` false))))))

(event `EnhancedInput|/Game/leBaguette/Paul/Input/Actions/IA_AttackRange`
  (params (ActionValue :type Boolean) (ElapsedSeconds :type "Float (double-precision)") (TriggeredSeconds :type "Float (double-precision)") (InputAction :type "InputAction Object Reference" :default "/Game/leBaguette/Paul/Input/Actions/IA_AttackRange.IA_AttackRange"))
  (bind (_bullet _speed _damagemultiplier) (break `/Game/leBaguette/Joa/Struct/Struct_Bullet` (`|GetArrayItem` (`/Game/leBaguette/Joa/DataAssets/Inventory/DA_RangeWeapon.Combos` (`self.EquippedRange`)) (`self.RangeCurrentCombo`))))
  (:`Triggered`
    (if (not (`self.RangeOnCooldown`))
      (`self.SpawnBullet` _bullet _damagemultiplier _speed)
      (set `self.RangeOnCombo` true)
      (set `self.RangeOnCooldown` true)
      (if (< (`self.RangeCurrentCombo`) (- (`KismetArrayLibrary.Array_Length` (`/Game/leBaguette/Joa/DataAssets/Inventory/DA_RangeWeapon.Combos` (`self.EquippedRange`))) 1))
        (`/Engine/EditorBlueprintResources/StandardMacros.IncrementInt` (`self.RangeCurrentCombo`)
          (:`  `
            _))
        (else
          (set `self.RangeCurrentCombo` 0)
          (set `self.RangeOnCombo` false)))
      (`|ExecutionSequence`
        (:`then_0`
          (`KismetSystemLibrary.Delay` (* (`/Game/leBaguette/Joa/DataAssets/Inventory/DA_Weapon.AttackRate` (`self.EquippedRange`)) (`self.AttackRateModifier`)))
          (set `self.RangeOnCooldown` false))
        (:`then_1`
          (`KismetSystemLibrary.Delay` (`self.ComboLasting`))
          (set `self.RangeCurrentCombo` 0)
          (set `self.RangeOnCombo` false))))))

(fn `CheckCubeCollider`
  (params (Extent :type "Vector Structure") (RelativePos :type "Vector Structure") (Damage :type "Float (double-precision)"))
  (bind _returnvalue (`self.GetOwner`))
  (bind _returnvalue_2 (+ (`Actor.K2_GetActorLocation` _returnvalue) (* (`Actor.GetActorRightVector` _returnvalue) (.x RelativePos)) (* (`Actor.GetActorForwardVector` _returnvalue) (.y RelativePos))))
  (bind _returnvalue_3 (`KismetMathLibrary.MakeRotator` (.roll (`Actor.K2_GetActorRotation` _returnvalue)) (.pitch (`Actor.K2_GetActorRotation` _returnvalue)) (+ (.yaw (`Actor.K2_GetActorRotation` _returnvalue)) 90.0)))
  (`KismetSystemLibrary.DrawDebugBox` _returnvalue_2 Extent (struct :`R` 1.0 :`G` 0.550446 :`B` 0.145359 :`A` 1.0) _returnvalue_3 5.0 5.0)
  (bind _outactors (`KismetSystemLibrary.BoxOverlapActorsWithOrientation` _returnvalue_2 Extent _returnvalue_3 (`|MakeArray` "ObjectTypeQuery1" "ObjectTypeQuery2" "ObjectTypeQuery3" :!type "EObjectTypeQuery Enum")))
  (for _array_element _outactors
    (if (`KismetSystemLibrary.DoesImplementInterface` _array_element "/Game/leBaguette/Joa/Interface/BPI_Attack.BPI_Attack_C")
      (message `/Game/leBaguette/Joa/Interface/BPI_Attack.AttackByPlayer` _array_element (* (`local.Damage`) (`self.DamageBonus`))))))

(fn `SpawnBullet`
  (params (BulletBP :type "/Game/leBaguette/Joa/BP_Bullet Class Reference") (Damage :type "Float (double-precision)") (Speed :type "Float (double-precision)"))
  (bind _returnvalue (`self.GetOwner`))
  (bind _returnvalue_2 (`|SpawnActorFromClass` BulletBP (`Actor.GetTransform` _returnvalue) "Undefined" "MultiplyWithRoot" null null))
  (`/Game/leBaguette/Joa/BP_Bullet.Init` _returnvalue_2 (* (`self.DamageBonus`) (`local.Damage`)) (`Actor.GetActorForwardVector` _returnvalue) (* (`local.Speed`) 100.0)))