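; Buff system component that tracks active timed buffs and keeps a summed per-stat map of their modifiers.
; AddBuff registers the buff uniquely but adds its stats on every call, broadcasts UpdateBuff, then subtracts and removes it after its lifespan.
; A single retriggerable delay handles expiry, so overlapping calls restart it and only the latest buff gets removed.
; UpdateResume can rebuild totals from active buffs but is not called here.
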(event `AddBuff`
  (params (Buff :type "/Game/leBaguette/Joa/OldInventoryAndBuffs/OldDA_Buff Object Reference"))
  (bind _activebuffs (`self.ActiveBuffs`))
  (if (not (`KismetArrayLibrary.Array_Contains` _activebuffs Buff))
    (`KismetArrayLibrary.Array_AddUnique` _activebuffs Buff))
  (`self.AddToResume` (`/Game/leBaguette/Joa/OldInventoryAndBuffs/OldDA_Buff.Stats` Buff))
  (`self.UpdateBuff`)
  (`KismetSystemLibrary.RetriggerableDelay` (`/Game/leBaguette/Joa/OldInventoryAndBuffs/OldDA_Buff.LifeSpan` Buff))
  (`self.RemoveToResume` (`/Game/leBaguette/Joa/OldInventoryAndBuffs/OldDA_Buff.Stats` Buff))
  (`KismetArrayLibrary.Array_RemoveItem` (`self.ActiveBuffs`) Buff)
  (`self.UpdateBuff`))

(fn `AddToResume`
  (params (Buff :type "Map of /Game/leBaguette/Joa/OldInventoryAndBuffs/OldStruct_BuffStat Structure to Float (double-precision)"))
  (bind _buffstatsresume (`self.BuffStatsResume`))
  (bind (_keypin _valuepin) (`|MapForEach` Buff)
    (:`then`
      (bind (_value _returnvalue) (`BlueprintMapLibrary.Map_Find` (`self.BuffStatsResume`) _keypin))
      (if _returnvalue
        (`BlueprintMapLibrary.Map_Add` _buffstatsresume _keypin (+ _value _valuepin))
        (else
          (`BlueprintMapLibrary.Map_Add` _buffstatsresume _keypin _valuepin))))
    (:`CompletedPin`
      (return))))

(fn `RemoveToResume`
  (params (Buff :type "Map of /Game/leBaguette/Joa/OldInventoryAndBuffs/OldStruct_BuffStat Structure to Float (double-precision)"))
  (bind _buffstatsresume (`self.BuffStatsResume`))
  (bind (_keypin _valuepin) (`|MapForEach` Buff)
    (:`then`
      (bind (_value _returnvalue) (`BlueprintMapLibrary.Map_Find` (`self.BuffStatsResume`) _keypin))
      (if _returnvalue
        (bind _returnvalue_2 (- _value _valuepin))
        (if (!= _returnvalue_2 0.0)
          (`BlueprintMapLibrary.Map_Add` _buffstatsresume _keypin _returnvalue_2)
          (else
            (`BlueprintMapLibrary.Map_Remove` _buffstatsresume _keypin)))))
    (:`CompletedPin`
      (return))))

(fn `UpdateResume`
  (`BlueprintMapLibrary.Map_Clear` (`self.BuffStatsResume`))
  (for _array_element (`self.ActiveBuffs`)
    (`self.AddToResume` (`/Game/leBaguette/Joa/OldInventoryAndBuffs/OldDA_Buff.Stats` _array_element)))
  (return))