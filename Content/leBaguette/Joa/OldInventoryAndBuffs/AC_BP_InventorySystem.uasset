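; Inventory component that tracks owned weapons, buffs and ingredients, and handles equipping and crafting.
; Weapons form a unique list, equipped into melee or ranged slots after checking the type in the weapon Blueprint's class defaults.
; Buffs and ingredients are quantity maps whose removals fail rather than go negative.
; ProcessRecipe verifies every ingredient before consuming any, then grants the recipe's buff, weapon and ingredient outputs through the add functions.
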(fn `AddBuffs`
  (params (Buff :type "/Game/leBaguette/Joa/OldInventoryAndBuffs/DA_Buff Object Reference") (Quantity :type Integer))
  (returns (NewAmount :type Integer))
  (bind _possesedbuffs (`self.PossesedBuffs`))
  (bind _buff (`local.Buff`))
  (if (`BlueprintMapLibrary.Map_Contains` _possesedbuffs Buff)
    (`BlueprintMapLibrary.Map_Add` _possesedbuffs _buff (+ (`local.Quantity`) (`BlueprintMapLibrary.Map_Find` _possesedbuffs (`local.Buff`))))
    (else
      (`BlueprintMapLibrary.Map_Add` _possesedbuffs _buff (`local.Quantity`))))
  (return (`BlueprintMapLibrary.Map_Find` _possesedbuffs (`local.Buff`))))

(fn `AddIngredients`
  (params (Ingredient :type "/Game/leBaguette/Joa/OldInventoryAndBuffs/DA_InventoryEntry Object Reference (by ref)") (Quantity :type "Integer (by ref)"))
  (returns (NewAmount :type Integer))
  (bind _ingredient (`local.Ingredient`))
  (bind _possesedingredients (`self.PossesedIngredients`))
  (if (`BlueprintMapLibrary.Map_Contains` _possesedingredients Ingredient)
    (`BlueprintMapLibrary.Map_Add` _possesedingredients _ingredient (+ (`local.Quantity`) (`BlueprintMapLibrary.Map_Find` _possesedingredients (`local.Ingredient`))))
    (else
      (`BlueprintMapLibrary.Map_Add` _possesedingredients _ingredient (`local.Quantity`))))
  (return (`BlueprintMapLibrary.Map_Find` _possesedingredients (`local.Ingredient`))))

(fn `AddWeapon`
  (params (NewWeapon :type "/Game/leBaguette/Joa/OldInventoryAndBuffs/DA_Weapon Object Reference"))
  (returns (Added :type Boolean) (Index :type Integer))
  (`/Engine/EditorBlueprintResources/StandardMacros.IsValid` NewWeapon
    (:`Is Valid`
      (if (not (`KismetArrayLibrary.Array_Contains` (`self.PossesedWeapon`) (`local.NewWeapon`)))
        (bind _returnvalue (`KismetArrayLibrary.Array_AddUnique` (`self.PossesedWeapon`) (`local.NewWeapon`)))
        (return true _returnvalue)
        (else
          _)))
    (:`Is Not Valid`
      _))
  (return false -1))

(fn `EquipMelee`
  (params (Index :type Integer))
  (returns (Equipped :type Boolean) (NewMelee :type "/Game/leBaguette/Joa/OldInventoryAndBuffs/DA_Weapon Object Reference") (OldMelee :type "/Game/leBaguette/Joa/OldInventoryAndBuffs/DA_Weapon Object Reference"))
  (locals (_Weapon :type "/Game/leBaguette/Joa/OldInventoryAndBuffs/DA_Weapon Object Reference") (_OldMelee :type "/Game/leBaguette/Joa/OldInventoryAndBuffs/DA_Weapon Object Reference"))
  (if (< Index (`KismetArrayLibrary.Array_Length` (`self.PossesedWeapon`)))
    (bind _output_get (set `local._Weapon` (`|GetArrayItem` (`self.PossesedWeapon`) Index)))
    (if (`|EnumEquality` (defaults `Object` (`/Game/leBaguette/Joa/OldInventoryAndBuffs/DA_Weapon.WeaponBlueprint` _output_get)) "NewEnumerator0")
      (if (!= (`local._Weapon`) (`self.EquippedMelee`))
        (bind _output_get_2 (set `local._OldMelee` (`self.EquippedMelee`)))
        (bind _output_get_3 (set `self.EquippedMelee` (`local._Weapon`)))
        (return true _output_get_3 _output_get_2)
        (else
          _))))
  (return false "/Game/leBaguette/Joa/OldInventoryAndBuffs/Weapon/Weapons/DA_Sword01.DA_Sword01" "/Game/leBaguette/Joa/OldInventoryAndBuffs/Weapon/Weapons/DA_Sword01.DA_Sword01"))

(fn `EquipRange`
  (params (Index :type Integer))
  (returns (Equipped :type Boolean) (NewRange :type "/Game/leBaguette/Joa/OldInventoryAndBuffs/DA_Weapon Object Reference") (OldRange :type "/Game/leBaguette/Joa/OldInventoryAndBuffs/DA_Weapon Object Reference"))
  (locals (_Weapon :type "/Game/leBaguette/Joa/OldInventoryAndBuffs/DA_Weapon Object Reference") (_OldRange :type "/Game/leBaguette/Joa/OldInventoryAndBuffs/DA_Weapon Object Reference"))
  (if (< Index (`KismetArrayLibrary.Array_Length` (`self.PossesedWeapon`)))
    (bind _output_get (set `local._Weapon` (`|GetArrayItem` (`self.PossesedWeapon`) Index)))
    (if (`|EnumEquality` (defaults `Object` (`/Game/leBaguette/Joa/OldInventoryAndBuffs/DA_Weapon.WeaponBlueprint` _output_get)) "NewEnumerator1")
      (if (!= (`local._Weapon`) (`self.EquippedRange`))
        (bind _output_get_2 (set `local._OldRange` (`self.EquippedRange`)))
        (bind _output_get_3 (set `self.EquippedRange` (`local._Weapon`)))
        (return true _output_get_3 _output_get_2)
        (else
          _))))
  (return false "/Game/leBaguette/Joa/OldInventoryAndBuffs/Weapon/Weapons/DA_Sword01.DA_Sword01" "/Game/leBaguette/Joa/OldInventoryAndBuffs/Weapon/Weapons/DA_Sword01.DA_Sword01"))

(fn `ProcessRecipe`
  (params (Recipe :type "/Game/leBaguette/Joa/OldInventoryAndBuffs/Da_Recipes Object Reference"))
  (returns (Processed :type Boolean))
  (bind _inputs (`/Game/leBaguette/Joa/OldInventoryAndBuffs/Da_Recipes.Inputs` Recipe))
  (bind (_keypin _valuepin) (`|MapForEach` _inputs)
    (:`then`
      (bind (_value _returnvalue) (`BlueprintMapLibrary.Map_Find` (`self.PossesedIngredients`) _keypin))
      (if _returnvalue
        (if (not (>= _value _valuepin))
          (return false))
        (else
          (return false))))
    (:`CompletedPin`
      (bind (_keypin_2 _valuepin_2) (`|MapForEach` _inputs)
        (:`then`
          (`self.RemoveIngredients` _keypin_2 _valuepin_2))
        (:`CompletedPin`
          (bind (_keypin_3 _valuepin_3) (`|MapForEach` (`/Game/leBaguette/Joa/OldInventoryAndBuffs/Da_Recipes.OutputsBuff` (`local.Recipe`)))
            (:`then`
              (`self.AddBuffs` _keypin_3 _valuepin_3))
            (:`CompletedPin`
              (for _array_element (`/Game/leBaguette/Joa/OldInventoryAndBuffs/Da_Recipes.OutputsWeapon` (`local.Recipe`))
                (`self.AddWeapon` _array_element))
              (bind (_keypin_4 _valuepin_4) (`|MapForEach` (`/Game/leBaguette/Joa/OldInventoryAndBuffs/Da_Recipes.OutputsIngredients` (`local.Recipe`)))
                (:`then`
                  (`self.AddIngredients` _keypin_4 _valuepin_4))
                (:`CompletedPin`
                  (return true))))))))))

(fn `RemoveBuffs`
  (params (Buff :type "/Game/leBaguette/Joa/OldInventoryAndBuffs/DA_Buff Object Reference") (Quantity :type Integer))
  (returns (Removed :type Boolean) (NewAmount :type Integer))
  (locals (_NewAmount :type Integer))
  (bind _possesedbuffs (`self.PossesedBuffs`))
  (bind _buff (`local.Buff`))
  (if (`BlueprintMapLibrary.Map_Contains` _possesedbuffs Buff)
    (bind _output_get (set `local._NewAmount` (- (`BlueprintMapLibrary.Map_Find` _possesedbuffs _buff) (`local.Quantity`))))
    (if (>= _output_get 0)
      (`BlueprintMapLibrary.Map_Add` _possesedbuffs _buff _output_get)
      (return true (`local._NewAmount`))
      (else
        _)))
  (return false -1))

(fn `RemoveIngredients`
  (params (Ingredient :type "/Game/leBaguette/Joa/OldInventoryAndBuffs/DA_InventoryEntry Object Reference (by ref)") (Quantity :type "Integer (by ref)"))
  (returns (Removed :type Boolean) (NewAmount :type Integer))
  (locals (New_Amount :type Integer :default 0))
  (bind _possesedingredients (`self.PossesedIngredients`))
  (bind _ingredient (`local.Ingredient`))
  (if (`BlueprintMapLibrary.Map_Contains` _possesedingredients Ingredient)
    (bind _output_get (set `local.New_Amount` (- (`BlueprintMapLibrary.Map_Find` _possesedingredients _ingredient) (`local.Quantity`))))
    (if (>= _output_get 0)
      (`BlueprintMapLibrary.Map_Add` _possesedingredients _ingredient _output_get)
      (return true (`local.New_Amount`))
      (else
        _)))
  (return false -1))

(fn `RemoveWeaponIndex`
  (params (Index :type Integer))
  (returns (Removed :type Boolean) (WeaponEntry :type "/Game/leBaguette/Joa/OldInventoryAndBuffs/DA_Weapon Object Reference"))
  (locals (_OldWeapon :type "/Game/leBaguette/Joa/OldInventoryAndBuffs/DA_Weapon Object Reference"))
  (bind _possesedweapon (`self.PossesedWeapon`))
  (if (>= (`KismetArrayLibrary.Array_Length` _possesedweapon) Index)
    (bind _output_get (set `local._OldWeapon` (`|GetArrayItem` _possesedweapon Index)))
    (`KismetArrayLibrary.Array_Remove` _possesedweapon (`local.Index`))
    (return true _output_get)
    (else
      (return false "/Game/leBaguette/Joa/OldInventoryAndBuffs/Weapon/Weapons/DA_Sword01.DA_Sword01"))))

(fn `RemoveWeaponItem`
  (params (Item :type "/Game/leBaguette/Joa/OldInventoryAndBuffs/DA_Weapon Object Reference"))
  (returns (Removed :type Boolean))
  (if (`KismetArrayLibrary.Array_Contains` (`self.PossesedWeapon`) Item)
    (bind _returnvalue (`KismetArrayLibrary.Array_RemoveItem` (`self.PossesedWeapon`) (`local.Item`)))
    (return _returnvalue)
    (else
      (return false))))